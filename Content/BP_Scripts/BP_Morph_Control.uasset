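; BP_Morph_Control plays one Niagara skeletal-mesh morph effect, triggered by Sequencer frame, Sequencer event or pose order as EnumPlay selects.
; All triggers share a delayed path that requires PoseTurn to match MyOrder, picks the system by morph variant, activates it and calls OnActiveAnimation.
; Niagara exports particle data back, and when the first particle's Velocity-to-Position distance drops below MorphTime, it calls OnMorphFinished and deactivates the effect.
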(event `/Game/Interfaces/NewInterface.SequencerCurrentFrame`
  (params (sequencerCurrentFrame :type Integer))
  (switch `/Game/Niagara/experimenting/EnumPlay` (`self.enumPlay`)
    (:`NewEnumerator2`
      (if (`self.Iplayed`)
        _
        (elif (== (`self.StartPlayFrame`) sequencerCurrentFrame)
          (set `self.Iplayed` true)
          (`KismetSystemLibrary.PrintString` "Played by Time")
          (`KismetSystemLibrary.Delay` (`self.StartDelay`) :!label _label)
          (if (== (stale `/Game/Interfaces/NewInterface.PoseCounter` PoseTurn) (`self.MyOrder`))
            (`NiagaraComponent.SetVariableObject` (`self.Niagara`) "CallBack" self)
            (`KismetSystemLibrary.Delay` (`self.delay`))
            (switch `/Game/Niagara/experimenting/EnumNiagara_morph` (`self.enumMorphVar`)
              (:`NewEnumerator0`
                (`NiagaraComponent.SetAsset` (`self.Niagara`) "/Game/Niagara/experimenting/NS_Morph_SkeletalMesh_test.NS_Morph_SkeletalMesh_test" true))
              (:`NewEnumerator1`
                (`NiagaraComponent.SetAsset` (`self.Niagara`) "/Game/Niagara/experimenting/NS_Morph_SkeletalMesh_test_3.NS_Morph_SkeletalMesh_test_3" true))
              (:`NewEnumerator2`
                (`NiagaraComponent.SetAsset` (`self.Niagara`) "/Game/Niagara/experimenting/NS_Morph_SkeletalMesh_test_6.NS_Morph_SkeletalMesh_test_6" true)))
            (`ActorComponent.SetActive` (`self.Niagara`) true true)
            (`self.onActiveAnimation`)
            (`KismetSystemLibrary.PrintString` (`KismetStringLibrary.Conv_IntToString` sequencerCurrentFrame))))))))

(event `PlayBySequencer`
  (switch `/Game/Niagara/experimenting/EnumPlay` (`self.enumPlay`)
    (:`NewEnumerator1`
      (`KismetSystemLibrary.PrintString` (`KismetStringLibrary.Conv_IntToString` (stale `/Game/Interfaces/NewInterface.SequencerCurrentFrame` sequencerCurrentFrame)) true true (struct :`G` 0.059925 :`B` 1.0 :`A` 1.0) :!label _label_2)
      (goto _label))))

(event `/Game/Interfaces/NewInterface.PoseCounter`
  (params (PoseTurn :type Integer))
  (switch `/Game/Niagara/experimenting/EnumPlay` (`self.enumPlay`)
    (:`NewEnumerator0`
      (goto _label_2))))

(event `self.ReceiveBeginPlay`)

(event `self.ReceiveParticleData`
  (params (Data :type "Array of BasicParticleData Structure (by ref)") (NiagaraSystem :type "NiagaraSystem Object Reference") (SimulationPositionOffset :type "Vector Structure (by ref)"))
  (bind (_position _size _velocity) (break `BasicParticleData` (`|GetArrayItem` Data)))
  (bind _returnvalue (`KismetMathLibrary.VSize` (- _velocity _position)))
  (`KismetSystemLibrary.PrintString` (`KismetStringLibrary.Conv_DoubleToString` _returnvalue) true true (struct :`R` 0.941054 :`G` 0.940306 :`B` 1.0 :`A` 1.0))
  (if (< _returnvalue (`self.MorphTime`))
    (`self.onMorphFinished`)
    (`ActorComponent.SetActive` (`self.Niagara`) false false)))

(event `/Game/Interfaces/NewInterface.AnimationFinishedInterface`)

(fn `UserConstructionScript`)