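; BP_Morph is an actor that plays a staged Niagara morph effect around a skeletal mesh.
; PoseCounter runs it once if self-playing, or binds it to another object's morph-finished event when the turn matches its order.
; Enum-selected start, idle and end systems follow timed delays, notifying BP_GameMode mid-sequence.
; Optionally, the mesh then appears through a timeline-driven translucency material before receiving its final materials.
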(event `/Game/Interfaces/NewInterface.PoseCounter`
  (params (PoseTurn :type Integer))
  (bind (_returnvalue_location _returnvalue_rotation _returnvalue_scale) (`KismetMathLibrary.BreakTransform` (`self.GetTransform`)))
  (bind _ns_end (`self.NS_End`))
  (bind _ns_start (`self.NS_Start`))
  (bind _spawnscaling (`self.spawnScaling`))
  (bind _ns_idle (`self.NS_Idle`))
  (if (`self.PlayByItSelf`)
    (if (not (`self.IsPlayedOnce`))
      (set `self.IsPlayedOnce` true)
      (switch `/Game/Niagara/experimenting/EnumNiagaraStart` (`self.EnumNiagaraStart`) :!label _label
        (:`NewEnumerator0`
          (`NiagaraComponent.SetAsset` _ns_start "/Game/Niagara/experimenting/NS_test1.NS_test1" true))
        (:`NewEnumerator1`
          (`NiagaraComponent.SetAsset` _ns_start "/Game/Niagara/experimenting/NS_test1_2.NS_test1_2" true))
        (:`NewEnumerator2`
          (`NiagaraComponent.SetAsset` _ns_start "/Game/Niagara/experimenting/NS_test1_3.NS_test1_3" true)))
      (`ActorComponent.SetActive` (`self.NS_Start`) true false)
      (`KismetSystemLibrary.PrintString` "Active")
      (`KismetSystemLibrary.Delay` (`self.StartDelay`))
      (`KismetSystemLibrary.PrintString` "1" true true (struct :`R` 0.987612 :`G` 0.876889 :`B` 1.0 :`A` 1.0))
      (switch `/Game/Niagara/experimenting/NiagaraCustomEffects` (`self.NiagaraEnumSelection`)
        (:`NewEnumerator0`
          (`NiagaraComponent.SetVariableFloat` (`self.NS_Idle`) "User.spawnScaling" _spawnscaling)
          (`NiagaraComponent.SetAsset` (`self.NS_Idle`) "/Game/Niagara/experimenting/NS_test4.NS_test4" true))
        (:`NewEnumerator1`
          (`NiagaraComponent.SetVariableFloat` _ns_idle "User.spawnRateBP" _spawnscaling)
          (`NiagaraComponent.SetAsset` _ns_idle "/Game/Niagara/experimenting/NS_test2.NS_test2" true))
        (:`NewEnumerator2`
          (`NiagaraComponent.SetAsset` (`self.NS_Idle`) "/Game/Niagara/experimenting/NS_test4_3.NS_test4_3" true))
        (:`NewEnumerator3`
          (`NiagaraComponent.SetVariableFloat` (`self.NS_Idle`) "User.spawnRateBP" _spawnscaling)
          (`NiagaraComponent.SetAsset` (`self.NS_Idle`) "/Game/Niagara/experimenting/NS_test2_2.NS_test2_2" true)))
      (`KismetSystemLibrary.Delay` (`self.IdleDelay`))
      (`ActorComponent.SetActive` (`self.NS_Idle`) true false)
      (`KismetSystemLibrary.PrintString` "2" true true (struct :`R` 0.892471 :`G` 0.902395 :`B` 1.0 :`A` 1.0))
      (`ActorComponent.SetActive` (`self.NS_Start`) false false)
      (bind _outactors (`GameplayStatics.GetAllActorsOfClass` "/Game/BP_Scripts/BP_GameMode.BP_GameMode_C"))
      (`/Game/BP_Scripts/BP_GameMode.AnimationFinishedInterface` _outactors)
      (`KismetSystemLibrary.Delay` (`self.EndDelay`))
      (switch `/Game/Niagara/experimenting/EnumNiagaraDistroyed` (`self.EnumDistroyedSlection`)
        (:`NewEnumerator0`
          (`NiagaraComponent.SetAsset` (`self.NS_End`) "/Game/Niagara/NS_DianPose_End.NS_DianPose_End" true))
        (:`NewEnumerator2`
          (`NiagaraComponent.SetVariableFloat` (`self.NS_End`) "User.scaleOfMesh" (.x (.scale (`self.GetTransform`))))
          (`NiagaraComponent.SetVariableVec3` (`self.NS_End`) "User.scaleOfMeshVec" _returnvalue_scale)
          (`NiagaraComponent.SetAsset` (`self.NS_End`) "/Game/Niagara/NS_HengPose.NS_HengPose" true))
        (:`NewEnumerator3`
          (`NiagaraComponent.SetVariableFloat` (`self.NS_End`) "User.spawnRateBP" 700.0)
          (`NiagaraComponent.SetAsset` (`self.NS_End`) "/Game/Niagara/experimenting/NS_test2.NS_test2" true)))
      (`ActorComponent.SetActive` (`self.NS_Idle`) false true)
      (`ActorComponent.SetActive` (`self.NS_Start`) false true)
      (`KismetSystemLibrary.PrintString` "3" true true (struct :`R` 0.970537 :`G` 0.996008 :`B` 1.0 :`A` 1.0))
      (`ActorComponent.SetActive` (`self.NS_End`) true false)
      (`|ExecutionSequence`
        (:`then_0`
          (if (`self.SkeletalMeshV`)
            (bind _returnvalue (`KismetMaterialLibrary.CreateDynamicMaterialInstance` "/Game/Materials/M_Translusive.M_Translusive"))
            (`|ExecutionSequence`
              (:`then_0`
                (`PrimitiveComponent.SetMaterial` (`self.SkeletalMesh`) 0 _returnvalue)
                (`PrimitiveComponent.SetMaterial` (`self.SkeletalMesh`) 1 _returnvalue)
                (bind (_direction _newtrack_1) (`Timeline|Timeline`)
                  (:`Update`
                    (`MaterialInstanceDynamic.SetVectorParameterValue` _returnvalue "Translusiveness" (make `LinearColor` _newtrack_1)))
                  (:`Finished`
                    (`PrimitiveComponent.SetMaterial` (`self.SkeletalMesh`) 0 "/Engine/VREditor/UI/M_ContentWindow.M_ContentWindow")
                    (`PrimitiveComponent.SetMaterial` (`self.SkeletalMesh`) 1 "/Engine/EngineMeshes/BackgroundMaterial.BackgroundMaterial"))))
              (:`then_1`
                (`SceneComponent.SetVisibility` (`self.SkeletalMesh`) true false)
                (`ActorComponent.SetActive` (`self.NS_Idle`) false false :!label _label_2)
                (`ActorComponent.SetActive` (`self.NS_Start`) false false)))))
        (:`then_1`
          (`ActorComponent.SetActive` _ns_end false true)
          (`SceneComponent.SetHiddenInGame` _ns_end true false)
          (`KismetSystemLibrary.PrintString` "done!" true true (struct :`R` 0.995833 :`G` 1.0 :`B` 0.991666 :`A` 1.0))
          (goto _label_2))))
    (else
      (set `self.CurrentTurn` PoseTurn)
      (if (== PoseTurn (`self.MyOrder`))
        (add `/Game/BP_Scripts/BP_Morph_Control.onMorphFinished` (`self.OnAnimationActiveRefrence `) (delegate `StartAnimation`))))))

(event `self.ReceiveBeginPlay`)

(event `StartAnimation`
  (goto _label))

(event `Play the Animation`)

(event `GetTriggerSequencer`
  (if (`self.GetTrigger`)
    (`SceneComponent.SetWorldScale3D` (`self.SkeletalMesh`) (8.0 8.0 8.0))
    (`ActorComponent.SetActive` (`self.NS_Start`) true true)
    (`KismetSystemLibrary.Delay` 10.0)
    (`KismetSystemLibrary.Delay` (`self.EndDelay`))
    (`SceneComponent.SetVisibility` (`self.SkeletalMesh`) false false)))

(event `endAnimation`
  (`ActorComponent.SetActive` (`self.NS_End`) true false)
  (`ActorComponent.SetActive` (`self.NS_Start`) false false))

(fn `UserConstructionScript`)