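; BP_GameMode is a game mode that drives a pose counter for morph actors in the level.
; On BeginPlay it sends the current PoseTurn to BP_Morph_Control and BP_Morph actors through a PoseCounterMessage call.
; Each AnimationFinishedInterface event increments PoseTurn and repeats that broadcast, forming a loop that advances the poses in turn.
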(event `self.ReceiveBeginPlay`
  (bind _outactors (`GameplayStatics.GetAllActorsOfClass` "/Game/BP_Scripts/BP_Morph_Control.BP_Morph_Control_C" :!label _label))
  (message `/Game/Interfaces/NewInterface.PoseCounter` _outactors (`self.PoseTurn`))
  (bind _outactors_2 (`GameplayStatics.GetAllActorsOfClass` "/Game/BP_Scripts/BP_Morph.BP_Morph_C"))
  (message `/Game/Interfaces/NewInterface.PoseCounter` _outactors_2 (`self.PoseTurn`)))

(event `/Game/Interfaces/NewInterface.AnimationFinishedInterface`
  (set `self.PoseTurn` (+ (`self.PoseTurn`) 1))
  (`KismetSystemLibrary.PrintString` (`KismetStringLibrary.Conv_IntToString` (`self.PoseTurn`)) false false (struct :`R` 1.0 :`G` 0.111831 :`A` 1.0))
  (goto _label))

(fn `UserConstructionScript`)